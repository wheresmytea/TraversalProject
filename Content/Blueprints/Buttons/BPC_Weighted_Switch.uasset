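; BPC_Weighted_Switch is a pressure-plate switch that triggers a linked interactive object while something overlaps it.
; Begin and end overlap each cast ButtonPointer to Master_interaction and call SwitchInteraction on it, with no filter on the overlapping actor.
; The Press_Anim timeline then sweeps SwitchPlate's relative location, playing from start on entry and reversing from end on exit.
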(event Collision|EventActorEndOverlap
  (params (OtherActor :type Actor%20Object%20Reference))
  (bind _asmaster_interaction (Utilities|Casting|CastToMaster_interaction (Variables|Default|GetButton_Pointer)))
  (Default|SwitchInteraction _asmaster_interaction)
  (bind _press (Timeline|Press_Anim ReverseFromEnd)
    (:Update
      (Transformation|SetRelativeLocation (Variables|Default|GetSwitch_Plate) _press true false))))

(event Collision|EventActorBeginOverlap
  (params (OtherActor :type Actor%20Object%20Reference))
  (bind _asmaster_interaction (Utilities|Casting|CastToMaster_interaction (Variables|Default|GetButton_Pointer)))
  (Default|SwitchInteraction _asmaster_interaction)
  (bind _press (Timeline|Press_Anim PlayFromStart)
    (:Update
      (Transformation|SetRelativeLocation (Variables|Default|GetSwitch_Plate) _press true false))))

(fn ConstructionScript
  (|CallParentFunction))