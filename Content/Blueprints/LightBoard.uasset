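; LightBoard is a Blueprint with a set of five point lights that can be switched to green individually.
; Each custom event, Light1 through Light5, sets the color of its own point light to a slightly different shade of green.
; The file contains no logic to reset the colors, and the construction script only calls the parent.
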(event Custom|Light%203
  (Rendering|Components|Light|SetLightColor (Variables|Default|GetPointLight2) "(R=0.033557,G=0.500000,B=0.000000,A=1.000000)" true))

(event Custom|Light%201
  (Rendering|Components|Light|SetLightColor (Variables|Default|GetPointLight) "(R=0.041879,G=0.480000,B=0.000000,A=1.000000)" true))

(event Custom|Light%202
  (Rendering|Components|Light|SetLightColor (Variables|Default|GetPointLight1) "(R=0.023490,G=0.500000,B=0.000000,A=1.000000)" true))

(event Custom|Light%204
  (Rendering|Components|Light|SetLightColor (Variables|Default|GetPointLight3) "(R=0.000000,G=0.490000,B=0.026309,A=1.000000)" true))

(event Custom|Light%205
  (Rendering|Components|Light|SetLightColor (Variables|Default|GetPointLight4) "(R=0.063356,G=0.590000,B=0.000000,A=1.000000)" true))

(fn ConstructionScript
  (|CallParentFunction))