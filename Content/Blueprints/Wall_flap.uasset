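; Wall flap Blueprint that flips its Cylinder component between two fixed rotations with an instant, swept transform change.
; BeginPlay, SwitchInteraction and Interactwithobject share one toggle that reads and inverts CurrentState, so the flap also flips once at start.
; Direct interaction toggles it only when ExternalSwitch is false, while SwitchInteraction always does.
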(event EventSwitchInteraction
  (if (Variables|Default|Getcurrent%20State)
    (Transformation|SetRelativeLocationAndRotation (Variables|Default|GetCylinder) "0, 0, 0" "90.000000,90.000000,90.000000" true false)
    (Variables|Default|Setcurrent%20State false)
    (else
      (Transformation|SetRelativeLocationAndRotation (Variables|Default|GetCylinder) "0, 0, 0" "0,90.000000,90.000000" true false)
      (Variables|Default|Setcurrent%20State true))))

(event EventInteractwithobject
  (if (not (Variables|Default|GetExternal%20Switch))
    (if (Variables|Default|Getcurrent%20State)
      (Transformation|SetRelativeLocationAndRotation (Variables|Default|GetCylinder) "0, 0, 0" "90.000000,90.000000,90.000000" true false)
      (Variables|Default|Setcurrent%20State false)
      (else
        (Transformation|SetRelativeLocationAndRotation (Variables|Default|GetCylinder) "0, 0, 0" "0,90.000000,90.000000" true false)
        (Variables|Default|Setcurrent%20State true)))))

(event EventBeginPlay
  (if (Variables|Default|Getcurrent%20State)
    (Transformation|SetRelativeLocationAndRotation (Variables|Default|GetCylinder) "0, 0, 0" "90.000000,90.000000,90.000000" true false)
    (Variables|Default|Setcurrent%20State false)
    (else
      (Transformation|SetRelativeLocationAndRotation (Variables|Default|GetCylinder) "0, 0, 0" "0,90.000000,90.000000" true false)
      (Variables|Default|Setcurrent%20State true))))

(fn ConstructionScript
  (|CallParentFunction))